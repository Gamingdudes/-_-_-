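; Base gun Blueprint whose Shoot function fires a hitscan shot; its other graphs are empty.
; A visibility line trace between the supplied points drives dirt impact, muzzle flash and damage on a hit.
; A second trace, with no End set, starts at the muzzle, supplies the flash and sound location, and re-enters the same hit branch, which still tests the first trace.
; The sound plays regardless of a hit.
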(fn `shoot`
  (params (Startlocation :type "Vector Structure") (Endlocation :type "Vector Structure") (Bulletstart :type "Vector Structure") (Bulletfirerotator :type "Rotator Structure"))
  (`|ExecutionSequence`
    (:`then_0`
      (bind (_outhit _returnvalue) (`KismetSystemLibrary.LineTraceSingle` Startlocation Endlocation "TraceTypeQuery1"))
      (if _returnvalue :!label _label
        (bind (_bblockinghit _binitialoverlap _time _distance _location _impactpoint _normal _impactnormal _physmat _hitactor) (`GameplayStatics.BreakHitResult` _outhit))
        (`GameplayStatics.SpawnEmitterAtLocation` "/Game/FPS_Weapons_Pack/Effects/ParticlesSystems/Impacts/Enviroment/P_Dirt_Impact.P_Dirt_Impact" _location)
        (bind (_bblockinghit_2 _binitialoverlap_2 _time_2 _distance_2 _location_2 _impactpoint_2 _normal_2 _impactnormal_2 _physmat_2 _hitactor_2 _hitcomponent _hitbonename _hititem _faceindex _tracestart) (`GameplayStatics.BreakHitResult` (stale _outhit_2)))
        (`GameplayStatics.SpawnEmitterAtLocation` "/Game/FPS_Weapons_Pack/Effects/ParticlesSystems/Weapons/KA47/P_KA47_Wide_and_Point_MF.P_KA47_Wide_and_Point_MF" _tracestart Bulletfirerotator)
        (`GameplayStatics.ApplyDamage` _hitactor (`self.Damage`))))
    (:`then_1`
      (bind _outhit_2 (`KismetSystemLibrary.LineTraceSingle` Bulletstart (0.0 0.0 0.0) "TraceTypeQuery1"))
      (goto _label))
    (:`then_2`
      (`GameplayStatics.PlaySoundAtLocation` "/Game/weaponsystem/fun/hehe_-_boy.hehe_-_boy" _tracestart))))

(fn `UserConstructionScript`)